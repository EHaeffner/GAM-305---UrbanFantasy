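; BP_Key is a trigger actor that opens matching doors when the third-person player character overlaps its box.
; On overlap it scans all Door_BP actors, opens each one sharing its ID, stores it as the last opened door, then plays a sound and prints a message.
; The end-overlap handler checks that stored door's validity but takes no further action.
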(event `self.Box.OnComponentBeginOverlap`
  (params (OverlappedComponent :type "PrimitiveComponent Object Reference") (OtherActor :type "Actor Object Reference") (OtherComp :type "PrimitiveComponent Object Reference") (OtherBodyIndex :type Integer) (bFromSweep :type Boolean) (SweepResult :type "HitResult Structure (by ref)"))
  (cast `/Game/ThirdPerson/Blueprints/BP_ThirdPersonCharacter` OtherActor)
  (bind _outactors (`GameplayStatics.GetAllActorsOfClass` "/Game/Assets/Door_BP.Door_BP_C"))
  (for _array_element _outactors
    (if (== (`/Game/Assets/Door_BP.ID` _array_element) (`self.ID`))
      (`/Game/Assets/Door_BP.OpenDoor` _array_element)
      (set `self.Last Opened Door` _array_element)
      (`GameplayStatics.PlaySound2D` "/Game/StarterContent/Audio/Untitled_video_-_Made_with_Clipchamp__1__Cue.Untitled_video_-_Made_with_Clipchamp__1__Cue" 1.0 1.0 0.0 null null)
      (`KismetSystemLibrary.PrintText` "A Door have opened."))))

(event `self.Box.OnComponentEndOverlap`
  (params (OverlappedComponent :type "PrimitiveComponent Object Reference") (OtherActor :type "Actor Object Reference") (OtherComp :type "PrimitiveComponent Object Reference") (OtherBodyIndex :type Integer))
  (cast `/Game/ThirdPerson/Blueprints/BP_ThirdPersonCharacter` OtherActor)
  (`/Engine/EditorBlueprintResources/StandardMacros.IsValid` (`self.Last Opened Door`)))

(fn `UserConstructionScript`)