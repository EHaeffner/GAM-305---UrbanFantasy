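; BP_Sword is a sword actor that animates its own size and can switch on a Hurty collider, likely for dealing damage.
; On BeginPlay it disables collision on the Sword component and runs a timeline in reverse to drive that component's scale.
; The Expand event enables query-only collision on Hurty and plays a second timeline that drives the same scale.
; No overlap or damage handling is implemented here.
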(event `self.ReceiveBeginPlay`
  (`PrimitiveComponent.SetCollisionEnabled` (`self.Sword`) "NoCollision")
  (bind (_direction _scale) (`Timeline|Timeline` :!via `Reverse`)
    (:`Update`
      (`SceneComponent.SetRelativeScale3D` (`self.Sword`) (`KismetMathLibrary.Conv_DoubleToVector` _scale)))))

(event `Expand`
  (`PrimitiveComponent.SetCollisionEnabled` (`self.Hurty`) "QueryOnly")
  (bind (_direction _scale) (`Timeline|Timeline_0`)
    (:`Update`
      (`SceneComponent.SetRelativeScale3D` (`self.Sword`) (`KismetMathLibrary.Conv_DoubleToVector` _scale)))))

(fn `UserConstructionScript`)