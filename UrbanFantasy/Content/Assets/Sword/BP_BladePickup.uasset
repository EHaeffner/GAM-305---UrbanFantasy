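; BP_BladePickup is a blade pickup that floats and spins until the player collects it.
; A looping timer calls Rotate to yaw the root, while the Bobbing timeline adds its value as a vertical local offset on each update.
; When BP_ThirdPersonCharacter overlaps the Sphere, the pickup calls WeaponCollect on the character and destroys itself.
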(event `self.ReceiveBeginPlay`
  ; Add floatiness and rotation
  (`KismetSystemLibrary.K2_SetTimer` null "Rotate" 0.005 true)
  (bind (_direction _float) (`Timeline|Bobbing`)
    (:`Update`
      (`SceneComponent.K2_AddLocalOffset` (`self.DefaultSceneRoot`) (`KismetMathLibrary.MakeVector` 0.0 0.0 _float) false false))))

(event `self.Sphere.OnComponentBeginOverlap`
  (params (OverlappedComponent :type "PrimitiveComponent Object Reference") (OtherActor :type "Actor Object Reference") (OtherComp :type "PrimitiveComponent Object Reference") (OtherBodyIndex :type Integer) (bFromSweep :type Boolean) (SweepResult :type "HitResult Structure (by ref)"))
  ; Overlap player to pickup
  (bind _asbp_third_person_character (cast `/Game/ThirdPerson/Blueprints/BP_ThirdPersonCharacter` OtherActor))
  (`/Game/ThirdPerson/Blueprints/BP_ThirdPersonCharacter.WeaponCollect` _asbp_third_person_character)
  (`self.K2_DestroyActor`))

(fn `Rotate`
  (`SceneComponent.K2_AddLocalRotation` (`self.DefaultSceneRoot`) (`KismetMathLibrary.MakeRotator` 0.0 0.0 0.5) false false))

(fn `UserConstructionScript`)