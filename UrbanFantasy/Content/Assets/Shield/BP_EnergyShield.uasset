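; Energy shield actor that blocks Projectile_BP hits by disabling their damage and destroying them, with a sound and brightness pulse.
; Activate and Deactivate toggle the DeflectionArea's query collision and animate the mesh scale, with the shield starting hidden and inactive.
; One timeline drives both animations, playing forward to shrink and, after a short delay, in reverse to expand.
; A dynamic material created in the construction script carries the pulse.
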(event `self.ReceiveBeginPlay`
  ; Have shield deactivated without shrink animation
  (`SceneComponent.SetRelativeScale3D` (`self.ShieldMesh`) (0.0 0.0 0.0))
  (`PrimitiveComponent.SetCollisionEnabled` (`self.DeflectionArea`) "NoCollision"))

(event `self.DeflectionArea.OnComponentBeginOverlap`
  (params (OverlappedComponent :type "PrimitiveComponent Object Reference") (OtherActor :type "Actor Object Reference") (OtherComp :type "PrimitiveComponent Object Reference") (OtherBodyIndex :type Integer) (bFromSweep :type Boolean) (SweepResult :type "HitResult Structure (by ref)"))
  ; Section to actually deflect projectiles once they've been added
  (bind _asprojectile_bp (cast `/Game/Assets/Projectile_BP` OtherActor))
  (`/Game/Assets/Projectile_BP.Disable Damage` _asprojectile_bp)
  (`self.Pulse`)
  (`GameplayStatics.PlaySoundAtLocation` "/Game/StarterContent/Audio/Explosion01.Explosion01" (`self.K2_GetActorLocation`) (struct) 1.0 1.0 0.0 null null null null)
  (`self.K2_DestroyActor` _asprojectile_bp))

(event `Pulse`
  ; Pulse animation when deflecting
  (bind (_direction _poweralpha) (`Timeline|PulseTimeline` :!via `PlayFromStart`)
    (:`Update`
      (`MaterialInstanceDynamic.SetScalarParameterValue` (`self.Shield Material`) "Brightness" (`KismetMathLibrary.Lerp` 3.0 120.0 _poweralpha)))))

(event `Activate`
  ; Setting collision detection on/off when called, plus calling animation
  (`PrimitiveComponent.SetCollisionEnabled` (`self.DeflectionArea`) "QueryOnly")
  (`self.ExpandShield`))

(event `Deactivate`
  ; Setting collision detection on/off when called, plus calling animation
  (`PrimitiveComponent.SetCollisionEnabled` (`self.DeflectionArea`) "NoCollision")
  (`self.ShrinkShield`))

(event `ShrinkShield`
  ; Actual animation for expanding/shrinking shield
  (bind (_direction _scale) (`Timeline|Shrink Timeline` :!via `PlayFromStart` :!label _label)
    (:`Update`
      (`SceneComponent.SetRelativeScale3D` (`self.ShieldMesh`) (`KismetMathLibrary.Conv_DoubleToVector` _scale)))))

(event `ExpandShield`
  ; Actual animation for expanding/shrinking shield
  (`KismetSystemLibrary.Delay` 0.2)
  (goto _label :!via `ReverseFromEnd`))

(fn `UserConstructionScript`
  (bind _returnvalue (`PrimitiveComponent.CreateDynamicMaterialInstance` (`self.ShieldMesh`) 0 "/Game/Assets/Shield/EnergyShield.EnergyShield" "None"))
  (set `self.Shield Material` _returnvalue))