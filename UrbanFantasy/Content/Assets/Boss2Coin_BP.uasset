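; Collectible coin for the second boss stage that counts toward the win condition.
; It spins every tick, and overlapping its Coin component increments Boss2CoinPickups on BP_ThirdPersonCharacter, then destroys the coin.
; On the fifth pickup it instead disables the character's input, destroys the character and opens the UI_WinScreen level.
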(event `self.ReceiveBeginPlay`)

(event `self.Coin.OnComponentBeginOverlap`
  (params (OverlappedComponent :type "PrimitiveComponent Object Reference") (OtherActor :type "Actor Object Reference") (OtherComp :type "PrimitiveComponent Object Reference") (OtherBodyIndex :type Integer) (bFromSweep :type Boolean) (SweepResult :type "HitResult Structure (by ref)"))
  (bind _asbp_third_person_character (cast `/Game/ThirdPerson/Blueprints/BP_ThirdPersonCharacter` OtherActor))
  (bind _boss2coinpickups (`/Game/ThirdPerson/Blueprints/BP_ThirdPersonCharacter.Boss2CoinPickups` _asbp_third_person_character))
  (set `/Game/ThirdPerson/Blueprints/BP_ThirdPersonCharacter.Boss2CoinPickups` (+ _boss2coinpickups 1) _asbp_third_person_character)
  (if (== _boss2coinpickups 5)
    (`self.DisableInput` _asbp_third_person_character (`GameplayStatics.GetPlayerController` 0))
    (`self.K2_DestroyActor` _asbp_third_person_character)
    (`GameplayStatics.OpenLevel` "UI_WinScreen")
    (else
      (`self.K2_DestroyActor`))))

(event `self.ReceiveTick`
  (params (DeltaSeconds :type "Float (single-precision)"))
  (`self.K2_AddActorLocalRotation` (struct :`Yaw` 3.0)))

(fn `UserConstructionScript`)